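; Player character Blueprint (主角, protagonist) that automatically fires bullets from the start of play.
; BeginPlay starts a looping timer that repeatedly calls 发射子弹 (fire bullet) and stores its handle.
; Each shot spawns the configured bullet class at the ArrowComponent tagged 子弹位置 selected by an index variable, using its location and rotation.
; 停止发射子弹 (stop firing) clears and invalidates the timer.
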(event EventBeginPlay
  (bind _returnvalue (Utilities|Time|SetTimerbyFunctionName 0 "发射子弹" 0.2 true))
  (Variables|Default|Set子弹发射计时器 _returnvalue))

(event Collision|EventActorBeginOverlap
  (params (OtherActor :type Actor%20Object%20Reference)))

(event EventTick
  (params (DeltaSeconds :type Float%20%28single-precision%29)))

(fn ConstructionScript)

(fn 发射子弹
  (bind _returnvalue (Actor|GetComponentsbyTag "/Script/Engine.ArrowComponent" "子弹位置"))
  (bind _子弹发射位置序号 (Variables|Default|Get子弹发射位置序号))
  (bind _output (Utilities|Array|Get(acopy) _returnvalue _子弹发射位置序号))
  (bind _returnvalue_2 (Transformation|GetWorldTransform _output))
  (Game|SpawnActorfromClass (Variables|Default|Get子弹类型) (Math|Transform|MakeTransform (.location _returnvalue_2) (.rotation _returnvalue_2) "1.000000,1.000000,1.000000") "Undefined" "MultiplyWithRoot" 0 0))

(fn 停止发射子弹
  (Utilities|Time|ClearandInvalidateTimerbyHandle (Variables|Default|Get子弹发射计时器)))