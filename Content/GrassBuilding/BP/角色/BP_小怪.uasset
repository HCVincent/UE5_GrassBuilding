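; Minion enemy (BP_小怪) that chases BP_主角 with AI MoveTo and carries an attached grass-cutting actor (BP_割草工具).
; 扣血 spawns a damage-number actor, subtracts its floating value from health, then triggers 受击 or 死亡.
; Hits play timelines for material glow, knockback and scale shrink.
; Death removes knife and cutter, enables mesh physics, and animates glow and a delayed dissolve.
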(event Custom|向目标移动
  (Utilities|Time|SetTimerbyEvent (delegate Custom|向目标移动) 1.0 true)
  (Utilities|FlowControl|DoOnce false :!label _label
    (:Completed
      (bind _returnvalue (Actor|GetActorOfClass "/Game/GrassBuilding/BP/角色/BP_主角.BP_主角_C"))
      (AI|AIMoveTo self "0, 0, 0" _returnvalue 5.0 false
        (:then
          (goto _label Reset))))))

(event Custom|受击
  (bind _returnvalue (Transformation|GetActorLocation))
  (Utilities|FlowControl|Sequence
    (:then_0
      (bind _time (Timeline|FreTimeline PlayFromStart)
        (:Update
          (Rendering|Material|SetScalarParameterValueonMaterials (Variables|Character|GetMesh) "外发光强度" _time))))
    (:then_1
      (Variables|Default|Set当前位置 _returnvalue)
      (Variables|Default|Set后退到位置 (- _returnvalue (* (Transformation|GetActorForwardVector) (Variables|Default|Get后退距离))))
      (bind _time_2 (Timeline|后退Timeline PlayFromStart)
        (:Update
          (Transformation|SetActorLocation (Math|Vector|Lerp(Vector) (Variables|Default|Get当前位置) (Variables|Default|Get后退到位置) _time_2) false false))))
    (:then_2
      (bind _time_3 (Timeline|缩小Tmeline PlayFromStart)
        (:Update
          (Transformation|SetActorScale3D (Math|Vector|Lerp(Vector) (Variables|Default|Get默认大小) (Variables|Default|Get缩小后大小) _time_3)))))))

(event Custom|死亡
  (bind _mesh (Variables|Character|GetMesh))
  (Utilities|FlowControl|DoOnce false
    (:Completed
      (Utilities|FlowControl|Sequence
        (:then_0
          (Collision|SetCollisionEnabled (Variables|Collision|GetCapsuleComponent) "NoCollision")
          (Collision|SetCollisionEnabled _mesh "PhysicsOnly")
          (Physics|SetSimulatePhysics _mesh true)
          (Utilities|FlowControl|Delay 0.75)
          (bind _time (Timeline|Timeline_0 PlayFromStart)
            (:Update
              (Rendering|Material|SetScalarParameterValueonMaterials (Variables|Character|GetMesh) "溶解值" _time))))
        (:then_1
          (Components|DestroyComponent (Variables|Default|Get小刀))
          (Actor|DestroyActor (Variables|Default|Get割草))
          (bind _time_2 (Timeline|Timeline PlayFromStart)
            (:Update
              (Rendering|Material|SetScalarParameterValueonMaterials (Variables|Character|GetMesh) "外发光强度" _time_2))))))))

(event Custom|测试伤害
  (CallFunction|扣血 2e+01))

(event Custom|TargetMovement
  (Utilities|Time|SetTimerbyEvent (delegate Custom|TargetMovement) 1.0 true)
  (Utilities|FlowControl|DoOnce false :!label _label
    (:Completed
      (Variables|/Script/Engine.CharacterMovementComponent|SetMaxWalkSpeed (Variables|Character|GetCharacterMovement) (Math|Random|RandomFloatinRange 1e+02 6e+02))
      (bind _returnvalue (Actor|GetActorOfClass 0))
      (AI|AIMoveTo self "0, 0, 0" _returnvalue 5.0 false
        (:OnSuccess
          (goto _label Reset))))))

(event EventBeginPlay
  (bind _returnvalue (Transformation|GetActorScale3D))
  (bind _returnvalue_2 (Game|SpawnActorfromClass "/Game/GrassBuilding/BP/割草系统/BP_割草工具.BP_割草工具_C" (Math|Transform|MakeTransform (Transformation|GetActorLocation) "0, 0, 0" "1.000000,1.000000,1.000000") "Undefined" "MultiplyWithRoot" 0 0.7 1.5e+02 0))
  (bind _output_get (Variables|Default|Set割草 _returnvalue_2))
  (Transformation|AttachComponentToComponent _output_get (Variables|Character|GetMesh) "root" "SnapToTarget" "KeepWorld" "KeepWorld" true)
  (Variables|Default|Set当前血量 (Variables|Default|Get最大血量))
  (Variables|Default|Set默认大小 _returnvalue)
  (Variables|Default|Set缩小后大小 (* _returnvalue (Variables|Default|Get缩小比率)))
  (CallFunction|向目标移动))

(event Collision|EventActorBeginOverlap
  (params (OtherActor :type Actor%20Object%20Reference)))

(event EventTick
  (params (DeltaSeconds :type Float%20%28single-precision%29)))

(fn ConstructionScript)

(fn 扣血
  (params (伤害 :type Float%20%28double-precision%29))
  (bind _returnvalue (Game|SpawnActorfromClass "/Game/GrassBuilding/BP/伤害字体/BP_伤害数值.BP_伤害数值_C" (Math|Transform|MakeTransform (Transformation|GetWorldLocation (Variables|Default|Get受击数值生成位置)) "0, 0, 0" "1.000000,1.000000,1.000000") "Undefined" "MultiplyWithRoot" 0 伤害 0))
  (bind _output_get (Variables|Default|Set当前血量 (- (Variables|Default|Get当前血量) (Variables|/Game/GrassBuilding/BP/伤害字体/BP_伤害数值.BP_伤害数值_C|Get伤害浮动值 _returnvalue))))
  (if (<= _output_get 0.0)
    (CallFunction|死亡)
    (else
      (CallFunction|受击))))