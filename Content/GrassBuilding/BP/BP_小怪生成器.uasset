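; Minion spawner actor that spawns BP_小怪 in a grid formation, either at BeginPlay or after a configurable delay.
; When enabled, the construction script lays out a grid of arrow components around the actor's origin, jittering each X/Y position with a seeded random stream, and stores them in an array.
; At spawn time, each valid arrow's world location, raised slightly in Z, and rotation become a minion's spawn transform.
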(event Custom|生成小怪
  (for _array_element (Variables|Default|GetArr)
    (Utilities|IsValid _array_element
      (:Is%20Valid
        (Game|SpawnActorfromClass "/Game/GrassBuilding/BP/角色/BP_小怪.BP_小怪_C" (Math|Transform|MakeTransform (Math|Vector|MakeVector (.x (Transformation|GetWorldLocation _array_element)) (.y (Transformation|GetWorldLocation _array_element)) (+ (.z (Transformation|GetWorldLocation _array_element)) 88.0)) (Transformation|GetWorldRotation _array_element) "1.000000,1.000000,1.000000") "Undefined" "MultiplyWithRoot" 0 0)))))

(event EventBeginPlay
  (if (Variables|Default|Get是否开局生成小怪)
    _
    (else
      (Utilities|FlowControl|Delay (Variables|Default|Get生成时间))))
  (CallFunction|生成小怪))

(event Collision|EventActorBeginOverlap
  (params (OtherActor :type Actor%20Object%20Reference)))

(event EventTick
  (params (DeltaSeconds :type Float%20%28single-precision%29)))

(fn ConstructionScript
  (bind _偏移值 (Variables|Default|Get偏移值))
  (bind _随机种子 (Variables|Default|Get随机种子))
  (bind _数量 (Variables|Default|Get数量))
  (bind _returnvalue (- (.y _数量) 1))
  (bind _returnvalue_2 (- (.x _数量) 1))
  (if (Variables|Default|Get是否生成箭头)
    (for _index (range 0 _returnvalue_2)
      (for _index_2 (range 0 _returnvalue)
        (bind _returnvalue_3 (AddComponent|AddArrowComponent false (Math|Transform|MakeTransform (Math|Vector|MakeVector (Math|Random|RandomFloatinRangefromStream _随机种子 (- (.X (Math|Vector|BreakVector (- (Math|Vector|MakeVector (* _index (Variables|Default|Get间隔)) (* _index_2 (Variables|Default|Get间隔)) 0.0) (Math|Vector|MakeVector (* (/ _returnvalue_2 2) (Variables|Default|Get间隔)) (* (/ _returnvalue 2) (Variables|Default|Get间隔)) 0.0)))) _偏移值) (+ (.X (Math|Vector|BreakVector (- (Math|Vector|MakeVector (* _index (Variables|Default|Get间隔)) (* _index_2 (Variables|Default|Get间隔)) 0.0) (Math|Vector|MakeVector (* (/ _returnvalue_2 2) (Variables|Default|Get间隔)) (* (/ _returnvalue 2) (Variables|Default|Get间隔)) 0.0)))) _偏移值)) (Math|Random|RandomFloatinRangefromStream _随机种子 (- (.Y (Math|Vector|BreakVector (- (Math|Vector|MakeVector (* _index (Variables|Default|Get间隔)) (* _index_2 (Variables|Default|Get间隔)) 0.0) (Math|Vector|MakeVector (* (/ _returnvalue_2 2) (Variables|Default|Get间隔)) (* (/ _returnvalue 2) (Variables|Default|Get间隔)) 0.0)))) _偏移值) (+ (.Y (Math|Vector|BreakVector (- (Math|Vector|MakeVector (* _index (Variables|Default|Get间隔)) (* _index_2 (Variables|Default|Get间隔)) 0.0) (Math|Vector|MakeVector (* (/ _returnvalue_2 2) (Variables|Default|Get间隔)) (* (/ _returnvalue 2) (Variables|Default|Get间隔)) 0.0)))) _偏移值)) 0.0) "0, 0, 0" "1.000000,1.000000,1.000000")))
        (Utilities|Array|Add (Variables|Default|GetArr) _returnvalue_3)))))