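; BP_重力枪 is a gravity gun prop actor that bobs vertically in the level, with no pickup or firing logic in its graphs.
; On BeginPlay it caches its spawn location plus upper and lower points offset by 单向浮动.
; One timeline lifts it from spawn to the top, then two more alternate endlessly between top and bottom, each lerping the actor location.
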(event EventBeginPlay
  (bind _returnvalue (Transformation|GetActorLocation))
  (bind _单向浮动 (Variables|Default|Get单向浮动))
  (bind (_x _y _z) (Math|Vector|BreakVector _returnvalue))
  (Variables|Default|Set出生位置 _returnvalue)
  (Variables|Default|Set上升位置 (Math|Vector|MakeVector _x _y (+ _z _单向浮动)))
  (Variables|Default|Set下降位置 (Math|Vector|MakeVector _x _y (- _z _单向浮动)))
  (Transformation|SetActorLocation (Variables|Default|Get出生位置) false false)
  (bind _move (Timeline|Timeline PlayFromStart)
    (:Update
      (Transformation|SetActorLocation (Math|Vector|Lerp(Vector) (Variables|Default|Get出生位置) (Variables|Default|Get上升位置) _move) false false))
    (:Finished
      (bind _move_2 (Timeline|Timeline_0 Play)
        (:Update
          (Transformation|SetActorLocation (Math|Vector|Lerp(Vector) (Variables|Default|Get上升位置) (Variables|Default|Get下降位置) _move_2) false false))
        (:Finished
          (bind _move_3 (Timeline|Timeline_1 PlayFromStart)
            (:Update
              (Transformation|SetActorLocation (Math|Vector|Lerp(Vector) (Variables|Default|Get下降位置) (Variables|Default|Get上升位置) _move_3) false false))
            (:Finished
              (Timeline|Timeline_0 PlayFromStart))))))))

(event Collision|EventActorBeginOverlap
  (params (OtherActor :type Actor%20Object%20Reference)))

(event EventTick
  (params (DeltaSeconds :type Float%20%28single-precision%29)))

(fn ConstructionScript)