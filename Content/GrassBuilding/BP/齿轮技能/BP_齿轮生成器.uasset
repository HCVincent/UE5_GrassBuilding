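; Gear spawner for the gear skill (齿轮技能) that places a ring of BP_单个齿轮 actors around itself.
; The construction script builds 生成数量 arrow components evenly spaced in yaw on a fixed-radius circle, pointing outward, and stores them in 齿轮生成位置.
; The custom event 生成齿轮 spawns one gear at each arrow and attaches it there, so the arrows act as sockets.
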(event Custom|生成齿轮
  (for _array_element (Variables|Default|Get齿轮生成位置)
    (bind _returnvalue (Game|SpawnActorfromClass "/Game/GrassBuilding/BP/齿轮技能/BP_单个齿轮.BP_单个齿轮_C" (Math|Transform|MakeTransform (Transformation|GetWorldLocation _array_element) "0, 0, 0" "1.000000,1.000000,1.000000") "Undefined" "MultiplyWithRoot" 0 0))
    (Transformation|AttachComponentToComponent _returnvalue _array_element "None" "SnapToTarget" "KeepRelative" "KeepRelative" true)))

(event EventBeginPlay)

(event Collision|EventActorBeginOverlap
  (params (OtherActor :type Actor%20Object%20Reference)))

(event EventTick
  (params (DeltaSeconds :type Float%20%28single-precision%29)))

(fn ConstructionScript
  (Utilities|Array|Clear (Variables|Default|Get齿轮生成位置))
  (for _index (range 0 (- (Variables|Default|Get生成数量) 1))
    (bind _returnvalue (AddComponent|AddArrowComponent false (Math|Transform|MakeTransform (* (Math|Rotator|GetRotationXVector (Math|Rotator|MakeRotator 0.0 0.0 (Math|Conversions|ToFloat(Integer) (* _index (/ 360 (Variables|Default|Get生成数量)))))) 3e+02) (Math|Rotator|MakeRotator 0.0 0.0 (Math|Conversions|ToFloat(Integer) (* _index (/ 360 (Variables|Default|Get生成数量))))) "1.000000,1.000000,1.000000")))
    (Utilities|Array|Add (Variables|Default|Get齿轮生成位置) _returnvalue)))