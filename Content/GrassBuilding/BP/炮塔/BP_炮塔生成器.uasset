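; BP_炮塔生成器 is a turret spawner that places a ring of turrets around its own center.
; The Construction Script adds evenly spaced, outward-facing arrow components at a configurable count and radius, storing them as spawn points.
; The 生成炮塔 event spawns the chosen turret class at each arrow with a -90° yaw offset and set scale, then calls 炮塔生成 on each BP_炮塔父级 instance.
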(event Custom|生成炮塔
  (for _array_element (Variables|Default|Get炮塔生成位置)
    (bind _returnvalue (Game|SpawnActorfromClass (Variables|Default|Get生成炮塔类型) (Math|Transform|MakeTransform (Transformation|GetWorldLocation _array_element) (Math|Rotator|MakeRotator (.roll (Transformation|GetWorldRotation _array_element)) (.pitch (Transformation|GetWorldRotation _array_element)) (- (.yaw (Transformation|GetWorldRotation _array_element)) 9e+01)) (Math|Conversions|ToVector(Float) (Variables|Default|Get生成大小))) "Undefined" "MultiplyWithRoot" 0 0))
    (bind _asbp_炮塔父级 (Utilities|Casting|CastToBP_炮塔父级 _returnvalue))
    (Default|炮塔生成 _asbp_炮塔父级)))

(event EventBeginPlay)

(event Collision|EventActorBeginOverlap
  (params (OtherActor :type Actor%20Object%20Reference)))

(event EventTick
  (params (DeltaSeconds :type Float%20%28single-precision%29)))

(fn ConstructionScript
  (Utilities|Array|Clear (Variables|Default|Get炮塔生成位置))
  (for _index (range 0 (- (Variables|Default|Get生成数量) 1))
    (bind _returnvalue (AddComponent|AddArrowComponent false (Math|Transform|MakeTransform (* (Math|Rotator|GetRotationXVector (Math|Rotator|MakeRotator 0.0 0.0 (Math|Conversions|ToFloat(Integer) (* _index (/ 360 (Variables|Default|Get生成数量)))))) (Variables|Default|Get离中心的距离)) (Math|Rotator|MakeRotator 0.0 0.0 (Math|Conversions|ToFloat(Integer) (* _index (/ 360 (Variables|Default|Get生成数量))))) "1.000000,1.000000,1.000000")))
    (Utilities|Array|Add (Variables|Default|Get炮塔生成位置) _returnvalue)))