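; BP_城墙 is a city wall actor, filed under the turret assets, that grows up out of the ground when it spawns.
; BeginPlay stores the Cube's world scale, flattens it to zero height, then plays a Timeline that lerps the scale back to the original.
; Only the Z scale changes, and the overlap, Tick and construction script are empty.
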(event EventBeginPlay
  (bind _output_get (Variables|Default|Set初始大小 (Transformation|GetWorldScale (Variables|Default|GetCube))))
  (Variables|Default|Set地下时大小 (Math|Vector|MakeVector (.X (Math|Vector|BreakVector _output_get)) (.Y (Math|Vector|BreakVector _output_get)) 0.0))
  (Transformation|SetWorldScale3D (Variables|Default|GetCube) (Variables|Default|Get地下时大小))
  (Components|Timeline|SetPlayRate (Variables|Default|GetTimeline) (/ 1.0 1.0))
  (bind _time (Timeline|Timeline PlayFromStart)
    (:Update
      (Transformation|SetWorldScale3D (Variables|Default|GetCube) (Math|Vector|Lerp(Vector) (Variables|Default|Get地下时大小) (Variables|Default|Get初始大小) _time)))))

(event Collision|EventActorBeginOverlap
  (params (OtherActor :type Actor%20Object%20Reference)))

(event EventTick
  (params (DeltaSeconds :type Float%20%28single-precision%29)))

(fn ConstructionScript)