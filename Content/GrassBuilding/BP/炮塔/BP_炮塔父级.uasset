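; Parent Blueprint for turrets that rise into place and automatically fire at BP_小怪 minions.
; 炮塔生成 plays an effect and timeline to unfold the hidden turret, then starts a looping FUNC_检测小怪 timer, which 停止检测 clears.
; Detection sphere-traces pawns along the actor's right vector and targets the nearest minion.
; 攻击 yaws the hub toward it, spawns BP_炮弹 at every arrow component, then re-enables detection.
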(event Custom|炮塔生成
  (Components|Activation|SetActive (Variables|Default|Get人物出现1) true true)
  (Development|SetHiddeninGame (Variables|Default|GetSM_Cannon_1_Hub) false false)
  (Components|Timeline|SetPlayRate (Variables|Default|Get炮旋转Timeline) (/ 1.0 0.5))
  (bind _time (Timeline|炮旋转Timeline PlayFromStart)
    (:Update
      (Transformation|SetWorldRotation (Variables|Default|GetSM_Cannon_1_Turret) (Math|Rotator|Lerp(Rotator) (Variables|出生动画|Get地下时旋转) (Variables|出生动画|Get初始旋转) _time) false false)
      (Transformation|SetWorldScale3D (Variables|Default|GetSM_Cannon_1_Hub) (Math|Vector|Lerp(Vector) (Variables|出生动画|Get地下时大小) (Variables|出生动画|Get初始大小) _time)))
    (:Finished
      (bind _returnvalue (Utilities|Time|SetTimerbyFunctionName 0 "FUNC_检测小怪" 0.01 true))
      (Variables|Default|Set检测小怪Timer _returnvalue))))

(event Custom|攻击
  (Variables|Default|Set攻击初始旋转 (Transformation|GetWorldRotation (Variables|Default|GetSM_Cannon_1_Hub)))
  (Variables|Default|Set需要打击的旋转信息 (Math|Rotator|FindLookatRotation (Transformation|GetActorLocation) (Variables|Default|Get需要打击的位置信息)))
  (Components|Timeline|SetPlayRate (Variables|Default|Get攻击旋转Timeline) (/ 1.0 0.25))
  (bind _time (Timeline|攻击旋转Timeline PlayFromStart)
    (:Update
      (Transformation|SetWorldRotation (Variables|Default|GetSM_Cannon_1_Hub) (Math|Rotator|Lerp(Rotator) (Math|Rotator|MakeRotator (.Roll (Math|Rotator|BreakRotator (Variables|Default|Get攻击初始旋转))) (.Pitch (Math|Rotator|BreakRotator (Variables|Default|Get攻击初始旋转))) (.Yaw (Math|Rotator|BreakRotator (Variables|Default|Get攻击初始旋转)))) (Math|Rotator|MakeRotator (.Roll (Math|Rotator|BreakRotator (Variables|Default|Get攻击初始旋转))) (.Pitch (Math|Rotator|BreakRotator (Variables|Default|Get攻击初始旋转))) (- (.Yaw (Math|Rotator|BreakRotator (Variables|Default|Get需要打击的旋转信息))) 9e+01)) _time true) false false))
    (:Finished
      (for _array_element (Actor|GetComponentsByClass "/Script/Engine.ArrowComponent")
        (Game|SpawnActorfromClass "/Game/GrassBuilding/BP/角色子弹/BP_炮弹.BP_炮弹_C" (Math|Transform|MakeTransform (.location (Transformation|GetWorldTransform _array_element)) (.rotation (Transformation|GetWorldTransform _array_element)) "1.000000,1.000000,1.000000") "Undefined" "MultiplyWithRoot" 0 0)
        (Variables|Default|Set是否检测 true)))))

(event Custom|停止检测
  (Utilities|Time|ClearandInvalidateTimerbyHandle (Variables|Default|Get检测小怪Timer)))

(event EventBeginPlay
  (bind _sm_cannon_1_hub (Variables|Default|GetSM_Cannon_1_Hub))
  (bind _sm_cannon_1_hub_2 (Variables|Default|GetSM_Cannon_1_Hub))
  (bind _returnvalue (Transformation|GetWorldScale _sm_cannon_1_hub))
  (bind (_x _y) (Math|Vector|BreakVector _returnvalue))
  (bind _output_get (Variables|出生动画|Set初始旋转 (Transformation|GetWorldRotation (Variables|Default|GetSM_Cannon_1_Turret))))
  (Variables|出生动画|Set地下时旋转 (Math|Rotator|MakeRotator (- (.Roll (Math|Rotator|BreakRotator _output_get)) 1.6e+02) (.Pitch (Math|Rotator|BreakRotator _output_get)) (.Yaw (Math|Rotator|BreakRotator _output_get))))
  (Transformation|SetWorldRotation (Variables|Default|GetSM_Cannon_1_Turret) (Variables|出生动画|Get地下时旋转) false false)
  (Variables|出生动画|Set初始大小 _returnvalue)
  (Variables|出生动画|Set地下时大小 (Math|Vector|MakeVector _x _y 0.1))
  (Transformation|SetWorldScale3D _sm_cannon_1_hub_2 (Variables|出生动画|Get地下时大小))
  (Development|SetHiddeninGame _sm_cannon_1_hub_2 true false))

(event Collision|EventActorBeginOverlap
  (params (OtherActor :type Actor%20Object%20Reference)))

(event EventTick
  (params (DeltaSeconds :type Float%20%28single-precision%29)))

(fn ConstructionScript)

(fn FUNC检测小怪
  (bind _returnvalue (Transformation|GetActorLocation))
  (if (Variables|Default|Get是否检测)
    (bind (_outhits _returnvalue_2) (Collision|MultiSphereTraceForObjects _returnvalue (+ _returnvalue (* (Transformation|GetActorRightVector) (Variables|属性检测|Get检测长度))) (Variables|属性检测|Get检测半径) (Utilities|Array|MakeArray "ObjectTypeQuery3") false 0 "None"))
    (if _returnvalue_2
      (Utilities|Array|Clear (Variables|Default|Get检测到的小怪))
      (for _array_element _outhits
        (bind _asbp_小怪 (Utilities|Casting|CastToBP_小怪 (.HitActor (Collision|BreakHitResult _array_element))))
        (Utilities|Array|Add (Variables|Default|Get检测到的小怪) _asbp_小怪))
      (Variables|Default|Set需要打击的位置信息 (Transformation|GetActorLocation (.ReturnValue (Actor|FindNearestActor (Transformation|GetActorLocation) (Variables|Default|Get检测到的小怪)))))
      (Variables|Default|Set是否检测 false)
      (CallFunction|攻击))))