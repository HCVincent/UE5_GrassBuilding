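; Floating damage-number actor that displays a randomized, negated damage value through its UMG_伤害数值 widget component.
; On BeginPlay, 伤害属性 rolls roughly even odds between doubled red and normal yellow damage, adds random spread, and replaces non-positive results with a yellow 1.
; 变化属性 derives start/end offset, size and angle for a timeline that also drives opacity.
; A looping timer calls 动画属性 by name to push these animated values into the widget.
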(event EventBeginPlay
  (Utilities|Time|SetTimerbyFunctionName 0 "动画属性" 0.01 true)
  (CallFunction|伤害属性)
  (CallFunction|变化属性)
  (Components|Timeline|SetPlayRate (Variables|Default|Get动画Timeline) (/ 1.0 0.25))
  (bind (_direction _动画 _不透明度) (Timeline|动画Timeline PlayFromStart)
    (:Update
      (Variables|Default|Set位置偏移 (Math|Float|Lerp (Variables|Default|Get偏移前位置) (Variables|Default|Get偏移后位置) _动画))
      (Variables|Default|Set字体大小 (Math|Float|Lerp (Variables|Default|Get偏移前大小) (Variables|Default|Get偏移后大小) _动画))
      (Variables|Default|Set偏移角度 (Math|Float|Lerp (Variables|Default|Get偏移角度) (Variables|Default|Get偏移后角度) _动画))
      (Variables|Default|Set字体不透明度 _不透明度))))

(event Collision|EventActorBeginOverlap
  (params (OtherActor :type Actor%20Object%20Reference)))

(event EventTick
  (params (DeltaSeconds :type Float%20%28single-precision%29)))

(fn ConstructionScript)

(fn 数值&颜色
  (params (字体颜色 :type Linear%20Color%20Structure :default "(R=1.000000,G=0.800000,B=0.050000,A=1.000000)") (数值 :type Float%20%28single-precision%29))
  (bind _asumg_伤害数值 (Utilities|Casting|CastToUMG_伤害数值 (UserInterface|GetUserWidgetObject (Variables|Default|GetWidget))))
  (Variables|/Game/GrassBuilding/BP/伤害字体/UMG_伤害数值.UMG_伤害数值_C|Set字体颜色 _asumg_伤害数值 字体颜色)
  (Variables|/Game/GrassBuilding/BP/伤害字体/UMG_伤害数值.UMG_伤害数值_C|Set数值 _asumg_伤害数值 (* 数值 -1.0)))

(fn 伤害属性
  (bind _数值 (Variables|Default|Get数值))
  (bind _数值_2 (Variables|Default|Get数值))
  (bind _returnvalue (* _数值 2.0))
  (if (>= (Math|Random|RandomFloatinRange 1.0 1e+02) 5e+01)
    (bind _output_get (Variables|Default|Set伤害浮动值 (Math|Random|RandomFloatinRange (- _returnvalue 2e+01) (+ _returnvalue 2e+01))))
    (if (<= _output_get 0.0)
      (CallFunction|数值&颜色 "(R=1.000000,G=0.799103,B=0.049707,A=1.000000)" 1.0)
      (else
        (CallFunction|数值&颜色 "(R=1.000000,G=0.150142,B=0.000000,A=1.000000)" _output_get)))
    (else
      (bind _output_get_2 (Variables|Default|Set伤害浮动值 (Math|Random|RandomFloatinRange (- _数值_2 2e+01) (+ _数值_2 2e+01))))
      (if (<= _output_get_2 0.0)
        (CallFunction|数值&颜色 "(R=1.000000,G=0.800000,B=0.050000,A=1.000000)" 1.0)
        (else
          (CallFunction|数值&颜色 "(R=1.000000,G=0.800000,B=0.050000,A=1.000000)" _output_get_2))))))

(fn 动画属性
  (bind _asumg_伤害数值 (Utilities|Casting|CastToUMG_伤害数值 (UserInterface|GetUserWidgetObject (Variables|Default|GetWidget))))
  (Variables|/Game/GrassBuilding/BP/伤害字体/UMG_伤害数值.UMG_伤害数值_C|Set字体不透明度 _asumg_伤害数值 (Variables|Default|Get字体不透明度))
  (Variables|/Game/GrassBuilding/BP/伤害字体/UMG_伤害数值.UMG_伤害数值_C|Set偏移角度 _asumg_伤害数值 (Variables|Default|Get偏移角度))
  (Variables|/Game/GrassBuilding/BP/伤害字体/UMG_伤害数值.UMG_伤害数值_C|Set字体大小 _asumg_伤害数值 (Variables|Default|Get字体大小))
  (Variables|/Game/GrassBuilding/BP/伤害字体/UMG_伤害数值.UMG_伤害数值_C|Set位置偏移 _asumg_伤害数值 (Variables|Default|Get位置偏移)))

(fn 变化属性
  (bind _偏移角度 (Variables|Default|Get偏移角度))
  (bind _位置偏移 (Variables|Default|Get位置偏移))
  (bind _字体大小 (Variables|Default|Get字体大小))
  (Variables|Default|Set偏移前角度 _偏移角度)
  (Variables|Default|Set偏移后角度 (+ _偏移角度 15.0))
  (Variables|Default|Set偏移后位置 (+ _位置偏移 25.0))
  (Variables|Default|Set偏移前位置 (- _位置偏移 25.0))
  (Variables|Default|Set偏移后大小 (* _字体大小 0.8))
  (Variables|Default|Set偏移前大小 (* _字体大小 1.2)))