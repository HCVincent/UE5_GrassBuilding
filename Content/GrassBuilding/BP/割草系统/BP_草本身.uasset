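; BP_草本身 is the cuttable grass of the mowing system, built on static mesh instances.
; Its 割草 (mow) event takes a hit and a rate, then multiplies the Z scale of the hit instance by that rate.
; When the result falls below a threshold, it removes the instance and spawns a grass-burst particle above it, using the instance's local-space location as the world position.
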(event EventBeginPlay)

(event EventTick
  (params (DeltaSeconds :type Float%20%28single-precision%29)))

(event Event割草
  (params (Hit :type Hit%20Result%20Structure) (割草数率 :type Float%20%28double-precision%29))
  (bind _hititem (Collision|BreakHitResult Hit))
  (bind _outinstancetransform (Components|InstancedStaticMesh|GetInstanceTransform _hititem false))
  (bind (_x _y _z) (Math|Vector|BreakVector (.location _outinstancetransform)))
  (bind _returnvalue (* (.z (.scale _outinstancetransform)) 割草数率))
  (if (< _returnvalue 0.2)
    (Effects|SpawnEmitteratLocation "/Game/GrassBuilding/FX/草特效/P_爆出草.P_爆出草" (Math|Vector|MakeVector _x _y (+ _z 7e+01)))
    (Class|InstancedStaticMeshComponent|RemoveInstance _hititem)
    (else
      (Components|InstancedStaticMesh|UpdateInstanceTransform _hititem (Math|Transform|MakeTransform (.location _outinstancetransform) (.rotation _outinstancetransform) (Math|Vector|MakeVector (.x (.scale _outinstancetransform)) (.y (.scale _outinstancetransform)) _returnvalue)) false false false))))