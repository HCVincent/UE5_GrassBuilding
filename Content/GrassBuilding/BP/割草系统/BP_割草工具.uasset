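; Grass-cutting tool actor (割草工具) that cuts grass within a spherical range around itself.
; Every Tick it runs a multi sphere trace on the Visibility channel at its location, using the 割草范围 sphere's radius.
; Hit components implementing BP_割草蓝图接口 receive the 割草 message with the hit and the 割草数率 rate, leaving the actual cutting to them.
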(event EventBeginPlay)

(event Collision|EventActorBeginOverlap
  (params (OtherActor :type Actor%20Object%20Reference)))

(event EventTick
  (params (DeltaSeconds :type Float%20%28single-precision%29))
  (bind _returnvalue (Transformation|GetActorLocation))
  (bind (_outhits _returnvalue_2) (Collision|MultiSphereTraceByChannel _returnvalue _returnvalue (Variables|/Script/Engine.SphereComponent|GetSphereRadius (Variables|Default|Get割草范围)) "TraceTypeQuery1" false 0 "None"))
  (if _returnvalue_2
    (for _array_element _outhits
      (if (Utilities|DoesObjectImplementInterface (.HitComponent (Collision|BreakHitResult _array_element)) "/Game/GrassBuilding/BP/割草系统/BP_割草蓝图接口.BP_割草蓝图接口_C")
        (Class|BP割草蓝图接口|割草(Message) (.HitComponent (Collision|BreakHitResult _array_element)) _array_element (Variables|Default|Get割草数率))))))

(fn ConstructionScript)