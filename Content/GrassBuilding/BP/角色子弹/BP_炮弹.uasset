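; BP_炮弹 is a cannon shell that spawns a trail effect on BeginPlay and destroys itself after a short lifetime.
; When Sphere1 overlaps a BP_小怪, it spawns an explosion and sphere-traces pawns, damaging each BP_小怪 and shaking the camera per hit.
; A second Visibility sphere trace sends the grass-cutting interface message to hit components.
; Early destruction happens only if that trace hits something.
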(event OnComponentBeginOverlap(Sphere1)
  (params (OverlappedComponent :type Primitive%20Component%20Object%20Reference) (OtherActor :type Actor%20Object%20Reference) (OtherComp :type Primitive%20Component%20Object%20Reference) (OtherBodyIndex :type Integer) (bFromSweep :type Boolean) (SweepResult :type Hit%20Result%20Structure%20%28by%20ref%29))
  (bind _returnvalue (Transformation|GetActorLocation))
  (Utilities|Casting|CastToBP_小怪 OtherActor)
  (Effects|SpawnEmitteratLocation "/Game/GrassBuilding/FX/道具特效/P_Explosion.P_Explosion" (Transformation|GetActorLocation) "0, 0, 0" "0.800000,0.800000,0.800000")
  (bind _outhits (Collision|MultiSphereTraceForObjects (Transformation|GetActorLocation) "0, 0, 0" 1.5e+02 (Utilities|Array|MakeArray "ObjectTypeQuery3") false 0 "None"))
  (for _array_element _outhits
    (bind _asbp_小怪 (Utilities|Casting|CastToBP_小怪 (.HitActor (Collision|BreakHitResult _array_element))))
    (Default|扣血 _asbp_小怪 1e+02)
    (Camera|PlayWorldCameraShake 0 (Transformation|GetActorLocation) 0.0 3e+03))
  (bind (_outhits_2 _returnvalue_2) (Collision|MultiSphereTraceByChannel _returnvalue _returnvalue 1.5e+02 "TraceTypeQuery1" false 0 "None"))
  (if _returnvalue_2
    (for _array_element_2 _outhits_2
      (if (Utilities|DoesObjectImplementInterface (.HitComponent (Collision|BreakHitResult _array_element_2)) "/Game/GrassBuilding/BP/割草系统/BP_割草蓝图接口.BP_割草蓝图接口_C")
        (Class|BP割草蓝图接口|割草(Message) (.HitComponent (Collision|BreakHitResult _array_element_2)) _array_element_2 0.0)))
    (Actor|DestroyActor)))

(event EventBeginPlay
  (Niagara|SpawnSystematLocation "/Game/GrassBuilding/FX/子弹特效/NS_炮弹拖尾.NS_炮弹拖尾" (Transformation|GetActorLocation) (Transformation|GetActorRotation))
  (Utilities|FlowControl|Delay 2.0)
  (Actor|DestroyActor))

(event Collision|EventActorBeginOverlap
  (params (OtherActor :type Actor%20Object%20Reference)))

(event EventTick
  (params (DeltaSeconds :type Float%20%28single-precision%29)))

(fn ConstructionScript)